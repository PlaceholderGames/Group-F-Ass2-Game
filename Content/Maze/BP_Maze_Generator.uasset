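; Maze generator that builds a seeded, grid-based maze as instanced wall meshes in the Construction Script, with border and maze display toggles.
; It carves paths by random two-tile steps linked by bridge tiles, backtracking through unchecked path tiles when boxed in.
; Tiles are tracked as flat indices in arrays; unclaimed tiles become walls.
; Optional loop paths open random qualifying walls before SpawnInstances converts indices to grid positions.
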(event EventBeginPlay)

(event Collision|EventActorBeginOverlap
  (params (OtherActor :type Actor%20Object%20Reference)))

(event EventTick
  (params (DeltaSeconds :type Float%20%28single-precision%29)))

(fn ConstructionScript
  (CallFunction|PopulateBorders (Variables|Default|GetSize) (Variables|Default|GetBorderTiles))
  (if (Variables|Default|GetBShowBorder)
    (Utilities|SpawnInstances (Variables|Default|GetBorderTiles) (Variables|Default|GetSize) (Variables|Default|GetTile%20Size) "8.000000,8.000000,0.125000" (Variables|Components|GetWall)
      (:Finished
        _)))
  (if (Variables|Default|GetBShowMaze)
    (CallFunction|SetInitialTile)
    (while (Variables|Default|GetBCurrentFreeSide) :!label _label
      (CallFunction|PickNearbyTile))
    (Utilities|Array|Add (Variables|Default|GetCheckedTiles) (Variables|Default|GetCurrentTile))
    (CallFunction|BackTrack)
    (Utilities|ConvertLastBridge
      (:BridgesLeft
        (goto _label))
      (:NoBridgesLeft
        (CallFunction|PopulateWalls)
        (if (Variables|Default|GetAllowLoopPaths)
          (CallFunction|AddLoopPaths))
        (Utilities|SpawnInstances (Variables|Default|GetWalls) (Variables|Default|GetSize) (Variables|Default|GetTile%20Size) "8.000000,8.000000,0.125000" (Variables|Components|GetWall))))))

(fn PopulateBorders
  (params (Size :type Integer) (BorderArray :type Array%20of%20Integers))
  (Variables|Default|SetL_Size Size)
  (for _index (range 0 (- (Variables|Default|GetL_Size) 1))
    (Utilities|Array|Add BorderArray _index))
  (for _index_2 (range 1 (- (Variables|Default|GetL_Size) 2))
    (Utilities|Array|Add BorderArray (+ (* _index_2 (Variables|Default|GetL_Size)) (- (Variables|Default|GetL_Size) 1))))
  (for _index_3 (range 1 (Variables|Default|GetL_Size))
    (Utilities|Array|Add BorderArray (+ (- _index_3 1) (* (Variables|Default|GetL_Size) (- (Variables|Default|GetL_Size) 1)))))
  (for _index_4 (range 1 (- (Variables|Default|GetL_Size) 2))
    (Utilities|Array|Add BorderArray (* _index_4 (Variables|Default|GetL_Size)))))

(fn SetInitialTile
  (Variables|Default|SetCurrentTile (+ (Variables|Default|GetSize) 1))
  (Utilities|Array|Add (Variables|Default|GetPathTiles) (Variables|Default|GetCurrentTile)))

(fn AddBridgePathTile
  (params (PathTile :type Integer) (BridgeTile :type Integer))
  (Utilities|Array|Add (Variables|Default|GetPathTiles) PathTile)
  (Variables|Default|SetCurrentTile PathTile)
  (Utilities|Array|Add (Variables|Default|GetBorderTiles) BridgeTile))

(fn PickNearbyTile
  (bind _size (Variables|Default|GetSize))
  (bind _currenttile (Variables|Default|GetCurrentTile))
  (bind _currenttile_2 (Variables|Default|GetCurrentTile))
  (bind _currenttile_3 (Variables|Default|GetCurrentTile))
  (bind _size_2 (Variables|Default|GetSize))
  (bind _currenttile_4 (Variables|Default|GetCurrentTile))
  (bind (_btileinarrays _pathtile _bridgetile) (Utilities|CheckEastTile _currenttile false))
  (bind (_btileinarrays_2 _pathtile_2 _bridgetile_2) (Utilities|CheckEastTile _currenttile_2 true))
  (bind (_btileinarrays_3 _pathtile_3 _bridgetile_3) (Utilities|CheckNorthTile _currenttile_3 _size_2 true))
  (bind (_btileinarrays_4 _pathtile_4 _bridgetile_4) (Utilities|CheckNorthTile _currenttile_4 _size false))
  (switch int (Math|Random|RandomIntegerinRangefromStream 0 3 (Variables|Default|GetRandomStream))
    (:0
      (if _btileinarrays_4 :!label _label
        (Utilities|CycleCounter (LocalVariables|GetCounter) 4
          (:True
            (if _btileinarrays_3 :!label _label_2
              (Utilities|CycleCounter (LocalVariables|GetCounter) 4
                (:False
                  (Variables|Default|SetBCurrentFreeSide false :!label _label_3)
                  (return)))
              (else
                (CallFunction|AddBridgePathTile _pathtile_3 _bridgetile_3))))
          (:False
            (goto _label_3)))
        (else
          (CallFunction|AddBridgePathTile _pathtile_4 _bridgetile_4))))
    (:1
      (if _btileinarrays
        (Utilities|CycleCounter (LocalVariables|GetCounter) 4
          (:True
            (if _btileinarrays_2 :!label _label_4
              (Utilities|CycleCounter (LocalVariables|GetCounter) 4
                (:True
                  (goto _label))
                (:False
                  (goto _label_3)))
              (else
                (CallFunction|AddBridgePathTile _pathtile_2 _bridgetile_2))))
          (:False
            (goto _label_3)))
        (else
          (CallFunction|AddBridgePathTile _pathtile _bridgetile))))
    (:2
      (goto _label_2))
    (:3
      (goto _label_4))))

(fn BackTrack
  (bind _arrayelement (Utilities|ForEachLoopwithBreak (Variables|Default|GetPathTiles) :!label _label)
    (:LoopBody
      (if (not (Utilities|Array|ContainsItem (Variables|Default|GetCheckedTiles) _arrayelement))
        (Variables|Default|SetCurrentTile _arrayelement)
        (goto _label Break)))))

(fn PopulateWalls
  (bind _size (Variables|Default|GetSize))
  (for _index (range 0 (- (* _size _size) 1))
    (if (not (Utilities|CheckTileArrays _index))
      (Utilities|Array|Add (Variables|Default|GetWallTiles) _index))))

(fn AddLoopPaths
  (LocalVariables|SetLoopPathsAdded 0)
  (LocalVariables|SetLoopPaths (Utilities|GetRandomArrayElement (Variables|Default|GetWallTiles) (Variables|Default|GetRandomStream)) :!label _label)
  (if (Utilities|TileSurrounded (LocalVariables|GetLoopPaths))
    _
    (else
      (Utilities|AddRemoveArrayItem (LocalVariables|GetLoopPaths) (Variables|Default|GetPathTiles) (Variables|Default|GetWallTiles)
        (:Out
          (LocalVariables|SetLoopPathsAdded (+ (LocalVariables|GetLoopPathsAdded) 1))))))
  (if (< (LocalVariables|GetLoopPathsAdded) (Variables|Default|GetMaxLoopPaths))
    (goto _label)))