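; Player character Blueprint for a 2D side-scroller that runs, jumps and fires projectiles.
; Input events set movement, falling and attacking flags, with touch mirroring jump and firing spawning ProjectileBP at a spawn component.
; Each tick, a function-based state machine picks the sprite flipbook from those flags, prioritizing attacking, then jumping, running and idle.
; The sprite flips to face the horizontal velocity, and landing clears the falling flag.
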(event Custom|Fire%20Projectile
  ;[1 1 1] Shooting
  (Game|SpawnActorfromClass "/Game/SpaceSucks/Blueprints/ProjectileBP.ProjectileBP_C" (Transformation|GetWorldTransform (Variables|Default|GetProjectilesSpawn)) "Undefined" 0 0)
  (Variables|Default|SetisAttacking true))

(event Custom|UpdateAnimation
  ;[1 1 1] Control Animation
  (Variables|Default|SetisMoving (> (Math|Vector|VectorLength (Transformation|GetVelocity)) 0.0))
  (bind _outputfb (CallFunction|AnimationStateMachine (Variables|Default|GetisMoving) (Variables|Default|GetisFalling) (Variables|Default|GetisAttacking)))
  (Sprite|SetFlipbook (Variables|Default|GetSprite) _outputfb))

(event EventTick
  (params (DeltaSeconds :type Float%20%28single-precision%29))
  ;[1 1 1] Sprite Rotation
  (CallFunction|UpdateAnimation)
  (Math|Float|CompareFloat (.X (Math|Vector|BreakVector (Variables|/Script/Engine.MovementComponent|GetVelocity (Variables|Character|GetCharacterMovement)))) 0.0
    (:>
      (Transformation|SetRelativeRotation (Variables|Default|GetSprite) "0, 0, 0" false false))
    (:<
      (Transformation|SetRelativeRotation (Variables|Default|GetSprite) "0,180.000000, 0" false false))))

(event EventOnLanded
  (params (Hit :type Hit%20Result%20Structure%20%28by%20ref%29))
  ;[1 1 1] Jumping
  (Variables|Default|SetisFalling false))

(event Input|ActionEvents|InputActionFire
  (params (Key :type Key%20Structure :default "AnyKey"))
  ;[1 1 1] Shooting
  (:Pressed
    (Variables|Default|SetisAttacking true)
    (CallFunction|FireProjectile)
    (Utilities|FlowControl|Delay 0.1)
    (Variables|Default|SetisAttacking false :!label _label))
  (:Released
    (goto _label)))

(event Input|ActionEvents|InputActionJump
  (params (Key :type Key%20Structure :default "AnyKey"))
  ;[1 1 1] Jumping
  (:Pressed
    (Character|Jump)
    (Variables|Default|SetisFalling true))
  (:Released
    (Character|StopJumping)))

(event Input|AxisEvents|InputAxisMoveRight
  (params (AxisValue :type Float%20%28single-precision%29))
  ;[1 1 1] Movement Control
  (Pawn|Input|AddMovementInput "1.000000, 0, 0" AxisValue false)
  (Variables|Default|SetisMoving true))

(event Input|TouchEvents|InputTouch
  (params (Location :type Vector) (FingerIndex :type ETouchIndex%20Enum))
  ;[1 1 1] Jumping
  (:Pressed
    (Character|Jump)
    (Variables|Default|SetisFalling true))
  (:Released
    (Character|StopJumping)))

(fn ConstructionScript)

(fn AnimationStateMachine
  (params (isMoving :type Boolean) (isFalling :type Boolean) (isAttacking :type Boolean))
  (if isAttacking
    (LocalVariables|SetAnimationState "NewEnumerator3")
    (elif isFalling
      (LocalVariables|SetAnimationState "NewEnumerator2")
      (elif isMoving
        (LocalVariables|SetAnimationState "NewEnumerator1")
        (else
          (LocalVariables|SetAnimationState "NewEnumerator0")))))
  (return (Utilities|Select :Index (LocalVariables|GetAnimationState) :NewEnumerator0 "/Game/Art/Sprites/Idle.Idle" :NewEnumerator1 "/Game/Art/Sprites/CharacterWalking.CharacterWalking" :NewEnumerator2 "/Game/Art/Sprites/Falling.Falling" :NewEnumerator3 "/Game/Art/Sprites/Shooting.Shooting")))